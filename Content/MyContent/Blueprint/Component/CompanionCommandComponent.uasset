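; CompanionCommandComponent stores a companion's current order and passes changes to its AI.
; On BeginPlay it caches the owner's BP_CompanionAIController.
; Follow, Hold, MoveTo and Watch functions set the command enum and the relevant target actor or location, with Watch storing its direction in the location variable.
; Each then sends an Event.Companion.Command.Changed event to the controller's StateTree component to signal the change.
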(event `self.ReceiveBeginPlay`
  (`|ExecutionSequence`
    (:`then_0`
      (bind _asbp_companion_aicontroller (cast `/Game/MyContent/Character/BP_CompanionAIController` (`AIBlueprintHelperLibrary.GetAIController` (`self.GetOwner`))))
      (set `self.Companion AIController` _asbp_companion_aicontroller))))

(fn `Command_Follow`
  (params (`Follow Actor` :type "Actor Object Reference"))
  (set `self.CurrentCommand` "NewEnumerator1")
  (set `self.CommandTargetActor` `Follow Actor`)
  (`self.Update State Tree`))

(fn `Command_Hold`
  (set `self.CurrentCommand` "NewEnumerator2")
  (set `self.CommandTargetActor` null)
  (`self.Update State Tree`))

(fn `Command_MoveTo`
  (params (`Move To Location` :type "Vector Structure"))
  (set `self.CurrentCommand` "NewEnumerator3")
  (set `self.CommandTargetLocation` `Move To Location`)
  (`self.Update State Tree`))

(fn `Command_Watch`
  (params (`Watch Direction` :type "Vector Structure"))
  (set `self.CurrentCommand` "NewEnumerator6")
  (set `self.CommandTargetLocation` `Watch Direction`)
  (`self.Update State Tree`))

(fn `Update State Tree`
  (`StateTreeComponent.SendStateTreeEvent` (`Actor.GetComponentByClass` (`self.Companion AIController`) "/Script/GameplayStateTreeModule.StateTreeComponent") (make `StateTreeEvent` (struct :`TagName` "Event.Companion.Command.Changed"))))