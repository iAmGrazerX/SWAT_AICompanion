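; BP_CompanionAIController is an AI controller for a companion that takes follow, hold, stop and move-to commands.
; Following stores a target and reissues MoveToActor through a looping timer calling RefreshFollowMove, with no Behavior Tree or Tick.
; Hold and stop both halt movement and clear the timer, but only stop clears the target.
; Move-to leaves the follow timer running, so an active follow can override it.
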(event `self.ReceiveBeginPlay`)

(fn `Command_FollowActor`
  (params (`New Follow Actor` :type "Actor Object Reference"))
  (`/Engine/EditorBlueprintResources/StandardMacros.IsValid` `New Follow Actor`
    (:`Is Valid`
      (set `self.Follow Target` (`local.New Follow Actor`))
      (`self.RefreshFollowMove`)
      (bind _returnvalue (`KismetSystemLibrary.K2_SetTimer` null "RefreshFollowMove" (`self.Follow Refresh Interval`) true))
      (set `self.Follow Referesh Timer Handle` _returnvalue))
    (:`Is Not Valid`
      (`self.Follow_Stop`))))

(fn `Command_Hold`
  (`self.StopMovement`)
  (`KismetSystemLibrary.K2_ClearAndInvalidateTimerHandle` (`self.Follow Referesh Timer Handle`))
  (`KismetSystemLibrary.PrintString` "Follow_Hold : Holding Current Position" false))

(fn `Command_MoveTo`
  (params (`Move To Location` :type "Vector Structure"))
  (`self.MoveToLocation` `Move To Location` 10.0 true true false true null))

(fn `Follow_Stop`
  (set `self.Follow Target` null)
  (`self.StopMovement`)
  (`KismetSystemLibrary.K2_ClearAndInvalidateTimerHandle` (`self.Follow Referesh Timer Handle`)))

(fn `RefreshFollowMove`
  (bind _follow_target (`self.Follow Target`)
    (:`then`
      (`self.MoveToActor` _follow_target 200.0 true true true null)
      (`KismetSystemLibrary.PrintString` "Follow_Move : Moving to Target" false))
    (:`else`)))

(fn `UserConstructionScript`)